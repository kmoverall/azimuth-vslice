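; SeasonNode is an actor that publishes its position and a size to the Nodes material parameter collection for materials to read.
; Its Index is appended to "Pos" and "Size" to pick the parameter slot it writes.
; Construction zeroes the size, and a timeline animates that parameter on BeginPlay, setting the Size variable when finished.
; Tick rewrites position and the Size variable to the collection every frame.
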(event EventTick
  (params (DeltaSeconds :type Float%20%28single-precision%29))
  (Rendering|Material|SetVectorParameterValue "/Game/Nodes.Nodes" (Utilities|String|StringToName (Utilities|String|Append "Pos" (Utilities|String|ToString(Integer) (Variables|Default|GetIndex)))) (Math|Conversions|ToLinearColor(Vector) (Transformation|GetActorLocation)) :!class /Script/Engine.KismetMaterialLibrary)
  (Rendering|Material|SetScalarParameterValue "/Game/Nodes.Nodes" (Utilities|String|StringToName (Utilities|String|Append "Size" (Utilities|String|ToString(Integer) (Variables|Default|GetIndex)))) (Variables|Default|GetSize) :!class /Script/Engine.KismetMaterialLibrary))

(event EventBeginPlay
  (bind _newtrack_5 (Timeline|Spawn_Timeline PlayFromStart)
    (:Update
      (Rendering|Material|SetScalarParameterValue "/Game/Nodes.Nodes" (Utilities|String|StringToName (Utilities|String|Append "Size" (Utilities|String|ToString(Integer) (Variables|Default|GetIndex)))) _newtrack_5 :!class /Script/Engine.KismetMaterialLibrary))
    (:Finished
      (Variables|Default|SetSize 1.5e+02))))

(fn ConstructionScript
  (Rendering|Material|SetScalarParameterValue "/Game/Nodes.Nodes" (Utilities|String|StringToName (Utilities|String|Append "Size" (Utilities|String|ToString(Integer) (Variables|Default|GetIndex)))) 0.0 :!class /Script/Engine.KismetMaterialLibrary)
  (Rendering|Material|SetVectorParameterValue "/Game/Nodes.Nodes" (Utilities|String|StringToName (Utilities|String|Append "Pos" (Utilities|String|ToString(Integer) (Variables|Default|GetIndex)))) (Math|Conversions|ToLinearColor(Vector) (Transformation|GetActorLocation)) :!class /Script/Engine.KismetMaterialLibrary))