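; Player character Blueprint for placing season nodes and switching the world's season.
; Number-slot inputs pick one of four seasons, and releasing the drop input spawns a SeasonNode at the character's location with that season, then pushes it to the AzimuthGame game mode.
; A separate input cycles the BaseSeason scalar in the Nodes material parameter collection through four values, changing the global season.
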(event Input|ActionEvents|InputActionDropNode
  (:Released
    (bind _returnvalue (Game|SpawnActorfromClass "/Game/Blueprints/SeasonNode.SeasonNode_C" (Math|Conversions|ToTransform(Vector) (Transformation|GetActorLocation)) true 0))
    (Variables|/Game/Blueprints/SeasonNode.SeasonNode_C|SetSeason _returnvalue (Variables|Default|GetSelectedSeason))
    (bind _asazimuth_game (Utilities|Casting|CastToAzimuthGame (Game|GetGameMode)))
    (Default|PushNodes _asazimuth_game _returnvalue)))

(event Input|ActionEvents|InputActionSetSeason0
  (:Pressed
    (Variables|Default|SetSelectedSeason 0)))

(event Input|ActionEvents|InputActionSetSeason1
  (:Pressed
    (Variables|Default|SetSelectedSeason 1)))

(event Input|ActionEvents|InputActionSetSeason2
  (:Pressed
    (Variables|Default|SetSelectedSeason 2)))

(event Input|ActionEvents|InputActionSetSeason3
  (:Pressed
    (Variables|Default|SetSelectedSeason 3)))

(event Input|ActionEvents|InputActionSwitchGlobalSeason
  (:Pressed
    (bind _returnvalue (Rendering|Material|GetScalarParameterValue "/Game/Nodes.Nodes" "BaseSeason" :!class /Script/Engine.KismetMaterialLibrary))
    (Rendering|Material|SetScalarParameterValue "/Game/Nodes.Nodes" "BaseSeason" (Math|Float|%(Float) (+ _returnvalue 1.0) 4.0) :!class /Script/Engine.KismetMaterialLibrary)))

(fn ConstructionScript)